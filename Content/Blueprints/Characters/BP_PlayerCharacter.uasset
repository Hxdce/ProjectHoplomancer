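; First-person player character with jumping, ledge mantling, smoothed crouching and a crosshair widget.
; Jump input also attempts a mantle, using traces for wall, walkable top and clearance, then moves the actor by a timeline rate-scaled to distance, with camera shake.
; A crouch timeline blends capsule height, camera height and walk speed; Tick reverses it upon release once a capsule trace finds headroom.
; Debug prints and trace drawing remain active.
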(event Input|EnhancedActionEvents|EnhancedInputActionIA_PlayerJump
  (params (ActionValue :type Boolean) (ElapsedSeconds :type Float%20%28double-precision%29) (TriggeredSeconds :type Float%20%28double-precision%29) (InputAction :type Input%20Action%20Object%20Reference :default "/Game/Input/IA_PlayerJump.IA_PlayerJump"))
  (:Started
    (Development|PrintString "Jump Start")
    (Character|Jump)
    (bind _canmantle (CallFunction|Mantle)) ; TODO: \n- Make mantle lerp time based on euclidean distance (Done?)\n- Make mantle only activate when player encounters a wall they can't easily jump over?\n- Possibly simplify code & improve hit detection?
    (if _canmantle
      (Class|LegacyCameraShake|StartLegacyCameraShake (Game|GetPlayerCameraManager 0) "/Game/Blueprints/Camera/BP_CameraShakeMantle.BP_CameraShakeMantle_C" 1.0 "CameraLocal" "0, 0, 0")
      (Variables|Default|SetInitialPlayerPosition (Transformation|GetActorLocation))
      (Variables|Default|SetDebug_TimeStart (Utilities|Time|GetTimeSeconds))
      (Components|Timeline|SetPlayRate (Variables|Default|GetMantleTime) (/ 1.0 (/ (Math|Vector|Distance(Vector) (Variables|Default|GetInitialPlayerPosition) (Variables|Default|GetFinalMantleTargetLocation)) 1e+02)))
      (bind _duration (Timeline|MantleTime PlayFromStart)
        (:Update
          (Transformation|SetActorLocation (Math|Vector|Lerp(Vector) (Variables|Default|GetInitialPlayerPosition) (Variables|Default|GetFinalMantleTargetLocation) _duration) false false)
          (Pawn|Components|CharacterMovement|SetMovementMode (Variables|Character|GetCharacterMovement) "MOVE_Walking" 0))
        (:Finished
          (bind _output_get (Variables|Default|SetDebug_TimeEnd (Utilities|Time|GetTimeSeconds)))
          (Development|PrintString (Utilities|String|ToString(Float) (/ (Math|Vector|Distance(Vector) (Variables|Default|GetInitialPlayerPosition) (Variables|Default|GetFinalMantleTargetLocation)) 1.0)))
          (Development|PrintString "Distance")
          (Development|PrintString (Utilities|String|ToString(Float) (- _output_get (Variables|Default|GetDebug_TimeStart))))
          (Development|PrintString "Time")
          (Development|PrintString (Utilities|String|ToString(Float) (/ (Math|Vector|Distance(Vector) (Variables|Default|GetInitialPlayerPosition) (Variables|Default|GetFinalMantleTargetLocation)) (- _output_get (Variables|Default|GetDebug_TimeStart)))))
          (Development|PrintString "Speed")))))
  (:Completed
    (Development|PrintString "Jump End")
    (Character|StopJumping)))

(event Input|EnhancedActionEvents|EnhancedInputActionIA_PlayerCrouch
  (params (ActionValue :type Boolean) (ElapsedSeconds :type Float%20%28double-precision%29) (TriggeredSeconds :type Float%20%28double-precision%29) (InputAction :type Input%20Action%20Object%20Reference :default "/Game/Input/IA_PlayerCrouch.IA_PlayerCrouch"))
  (:Started
    (Variables|Default|SetWantCrouch true)
    (bind _eyeheight (Timeline|CrouchStartTimeline Play)
      (:Update
        (Components|Capsule|SetCapsuleHalfHeight (Variables|Default|GetCapsuleComponent) (Math|Float|Lerp (Variables|Default|GetOriginalUncrouchedCapsuleHalfHeight) (Variables|Default|GetOriginalCrouchedCapsuleHalfHeight) _eyeheight) true)
        (Transformation|SetRelativeLocation (Variables|Default|GetPlayerCamera) (Math|Vector|MakeVector 0.0 0.0 (Math|Float|Lerp (Variables|Default|GetOriginalUncrouchedEyeHeight) (Variables|Default|GetOriginalCrouchedEyeHeight) _eyeheight)) false false)
        (Variables|/Script/Engine.CharacterMovementComponent|SetMaxWalkSpeed (Variables|Character|GetCharacterMovement) (Math|Float|Lerp (Variables|Default|GetTargetMoveSpeed) (Variables|Default|GetTargetCrouchSpeed) _eyeheight)))))
  (:Canceled
    (Variables|Default|SetWantCrouch false :!label _label))
  (:Completed
    (goto _label)))

(event EventBeginPlay
  (bind _charactermovement (Variables|Character|GetCharacterMovement))
  (bind _capsulecomponent (Variables|Default|GetCapsuleComponent))
  (bind _returnvalue (Components|Capsule|GetUnscaledCapsuleHalfHeight _capsulecomponent))
  (Variables|Default|SetOriginalUncrouchedCapsuleHalfHeight _returnvalue)
  (Variables|Default|SetOriginalCrouchedCapsuleHalfHeight (/ _returnvalue 2.0))
  (Variables|Default|SetTargetMoveSpeed (Variables|/Script/Engine.CharacterMovementComponent|GetMaxWalkSpeed _charactermovement))
  (Variables|Default|SetTargetCrouchSpeed (Variables|/Script/Engine.CharacterMovementComponent|GetMaxWalkSpeedCrouched _charactermovement))
  (Variables|Default|SetOriginalUncrouchedEyeHeight (Variables|Default|GetBaseEyeHeight))
  (Variables|Default|SetOriginalCrouchedEyeHeight (Variables|Default|GetCrouchedEyeHeight))
  (bind _returnvalue_2 (UserInterface|CreateWidget "/Game/Blueprints/UI/HUD/Crosshair.Crosshair_C"))
  (UserInterface|Viewport|AddtoViewport _returnvalue_2 0))

(event Collision|EventActorBeginOverlap
  (params (OtherActor :type Actor%20Object%20Reference)))

(event EventTick
  (params (DeltaSeconds :type Float%20%28single-precision%29))
  (if (< (Components|Capsule|GetScaledCapsuleHalfHeight (Variables|Default|GetCapsuleComponent)) (Variables|Default|GetOriginalUncrouchedCapsuleHalfHeight))
    (if (not (Variables|Default|GetWantCrouch))
      (bind _blocked (CallFunction|CheckifUncrouchBlocked))
      (if _blocked
        (bind _eyeheight (Timeline|CrouchStartTimeline Play)
          (:Update
            (Components|Capsule|SetCapsuleHalfHeight (Variables|Default|GetCapsuleComponent) (Math|Float|Lerp (Variables|Default|GetOriginalUncrouchedCapsuleHalfHeight) (Variables|Default|GetOriginalCrouchedCapsuleHalfHeight) _eyeheight) true)
            (Transformation|SetRelativeLocation (Variables|Default|GetPlayerCamera) (Math|Vector|MakeVector 0.0 0.0 (Math|Float|Lerp (Variables|Default|GetOriginalUncrouchedEyeHeight) (Variables|Default|GetOriginalCrouchedEyeHeight) _eyeheight)) false false)
            (Variables|/Script/Engine.CharacterMovementComponent|SetMaxWalkSpeed (Variables|Character|GetCharacterMovement) (Math|Float|Lerp (Variables|Default|GetTargetMoveSpeed) (Variables|Default|GetTargetCrouchSpeed) _eyeheight))))
        (else
          (Timeline|CrouchStartTimeline Reverse))))))

(fn ConstructionScript)

(fn CanJumpInternal
  (bind _returnvalue (|CallParentFunction))
  (if _returnvalue
    (return true)
    (else
      (return (and (Variables|Default|GetbIsCrouched) (not (AI|Components|NavMovement|IsFalling (Variables|Character|GetCharacterMovement))))))))

(fn CheckifUncrouchBlocked
  (bind _originaluncrouchedcapsulehalfheight (Variables|Default|GetOriginalUncrouchedCapsuleHalfHeight))
  (bind _capsulecomponent (Variables|Default|GetCapsuleComponent))
  (bind _returnvalue (Transformation|GetWorldLocation _capsulecomponent))
  (bind _returnvalue_2 (Components|Capsule|GetScaledCapsuleHalfHeight _capsulecomponent))
  (bind _returnvalue_3 (+ _originaluncrouchedcapsulehalfheight 2.0))
  (bind _returnvalue_4 (- _returnvalue (Math|Vector|MakeVector 0.0 0.0 _returnvalue_2)))
  (bind _returnvalue_5 (+ _returnvalue_4 (Math|Vector|MakeVector 0.0 0.0 _returnvalue_3)))
  (bind _outhit (Collision|CapsuleTraceByChannel _returnvalue_5 _returnvalue_5 (- (Components|Capsule|GetScaledCapsuleRadius _capsulecomponent) 2.0) (- _originaluncrouchedcapsulehalfheight 1.0) "TraceTypeQuery1" false 0 "None"))
  (return (.bBlockingHit (Collision|BreakHitResult _outhit))))

(fn Mantle
  (bind _returnvalue (Transformation|GetActorLocation))
  (bind _charactermovement (Variables|Character|GetCharacterMovement))
  (bind _maxmantleheight (Variables|Default|GetMaxMantleHeight))
  (bind _maxstepheight (Variables|/Script/Engine.CharacterMovementComponent|GetMaxStepHeight _charactermovement))
  (bind _returnvalue_2 (+ (.z _returnvalue) _maxstepheight))
  (bind _returnvalue_3 (Math|Vector|MakeVector (.x _returnvalue) (.y _returnvalue) _returnvalue_2))
  (Utilities|FlowControl|Sequence
    (:then_0
      ;[1 1 1] Check for blocking wall:
      (bind _outhit (Collision|CapsuleTraceByChannel _returnvalue_3 (+ _returnvalue_3 (* (Transformation|GetActorForwardVector) 32.0)) 32.0 (Variables|Default|GetOriginalUncrouchedCapsuleHalfHeight) "TraceTypeQuery1" false 0 "ForDuration"))
      (if (Math|Boolean|ANDBoolean (not (Class|CharacterMovementComponent|IsWalkable (Variables|Character|GetCharacterMovement) _outhit)) (.bBlockingHit (Collision|BreakHitResult _outhit)) (not (.bInitialOverlap (Collision|BreakHitResult _outhit))))
        (if (Utilities|IsValid (.HitActor (Collision|BreakHitResult _outhit)))
          (if (not (Physics|IsSimulatingPhysics (Variables|/Script/Engine.Actor|GetRootComponent (.HitActor (Collision|BreakHitResult _outhit))) "None"))
            _
            (else
              (return false))))
        (LocalVariables|SetInitialPoint (.ImpactPoint (Collision|BreakHitResult _outhit)))
        (LocalVariables|SetInitialNormal (.ImpactNormal (Collision|BreakHitResult _outhit)))
        (else
          (return false))))
    (:then_1
      ;[1 1 1] Trace downwards at surface target location
      (bind _outhit_2 (Collision|SphereTraceByChannel (+ (+ (Math|Vector|MakeVector (.x (LocalVariables|GetInitialPoint)) (.y (LocalVariables|GetInitialPoint)) (- (.z (LocalVariables|GetInitialPoint)) _maxmantleheight)) (* (LocalVariables|GetInitialNormal) -3e+01)) (Math|Vector|MakeVector 0.0 0.0 (* _maxmantleheight 2.0))) (+ (Math|Vector|MakeVector (.x (LocalVariables|GetInitialPoint)) (.y (LocalVariables|GetInitialPoint)) (- (.z (LocalVariables|GetInitialPoint)) _maxmantleheight)) (* (LocalVariables|GetInitialNormal) -3e+01)) 32.0 "TraceTypeQuery1" false 0 "ForDuration"))
      (if (and (Class|CharacterMovementComponent|IsWalkable (Variables|Character|GetCharacterMovement) _outhit_2) (.bBlockingHit (Collision|BreakHitResult _outhit_2)))
        (LocalVariables|SetTargetLocation (.Location (Collision|BreakHitResult _outhit_2)))
        (else
          (return false))))
    (:then_2
      ;[1 1 1] Check room & execute the mantle
      (bind _hasroom (CallFunction|CheckValidMantleLocation (LocalVariables|GetTargetLocation)))
      (if _hasroom
        (Pawn|Components|CharacterMovement|SetMovementMode (Variables|Character|GetCharacterMovement) "MOVE_None" 0)
        (Variables|Default|SetFinalMantleTargetLocation (Math|Vector|MakeVector (.x (LocalVariables|GetTargetLocation)) (.y (LocalVariables|GetTargetLocation)) (+ (.z (LocalVariables|GetTargetLocation)) (* (Components|Capsule|GetScaledCapsuleHalfHeight (Variables|Default|GetCapsuleComponent)) 0.5))))
        (return true)))))

(fn CheckValidMantleLocation
  (params (TargetLocation :type Vector))
  (bind _capsulecomponent (Variables|Default|GetCapsuleComponent))
  (bind _outhit (Collision|SphereTraceByChannel (Math|Vector|MakeVector (.x TargetLocation) (.y TargetLocation) (+ (.z TargetLocation) (Variables|/Script/Engine.CharacterMovementComponent|GetMaxStepHeight (Variables|Character|GetCharacterMovement)))) (Math|Vector|MakeVector (.x TargetLocation) (.y TargetLocation) (+ (.z TargetLocation) (Components|Capsule|GetScaledCapsuleHalfHeight _capsulecomponent))) (Components|Capsule|GetScaledCapsuleRadius _capsulecomponent) "TraceTypeQuery1" false 0 "None"))
  (return (Math|Boolean|NORBoolean (.bBlockingHit (Collision|BreakHitResult _outhit)) (.bInitialOverlap (Collision|BreakHitResult _outhit)))))