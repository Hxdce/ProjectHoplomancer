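; BP_FuncTest_Movement is a functional test checking that a character clears obstacles to reach a completion trigger.
; Each tick it moves the character forward and runs a short debug-drawn line trace ahead.
; A blocking hit fires a DoOnce that calls the character's jump-and-mantle handler twice with delays, then rearms.
; Overlapping the trigger reports success and returns the character to its recorded start location.
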(event OnActorBeginOverlap(CompletionTrigger)
  (params (OverlappedActor :type Actor%20Object%20Reference) (OtherActor :type Actor%20Object%20Reference))
  (bind _character (Variables|Default|GetCharacter))
  (if (== OtherActor _character)
    (Class|FunctionalTest|FinishTest "Succeeded" "Successfully cleared obstacles.")
    (Transformation|SetActorLocation _character (Variables|Default|GetCharacterStartLocation) false false)))

(event EventPrepareTest)

(event EventStartTest
  (Variables|Default|SetCharacterStartLocation (Transformation|GetActorLocation (Variables|Default|GetCharacter))))

(event EventTick
  (params (DeltaSeconds :type Float%20%28single-precision%29))
  (bind _character (Variables|Default|GetCharacter))
  (bind _character_2 (Variables|Default|GetCharacter))
  (bind _returnvalue (Transformation|GetActorForwardVector _character_2))
  (bind _returnvalue_2 (Transformation|GetActorLocation _character_2))
  (Pawn|Input|AddMovementInput _character_2 _returnvalue 1.0 false)
  (bind _outhit (Collision|LineTraceByChannel _returnvalue_2 (+ _returnvalue_2 (* _returnvalue 64.0)) "TraceTypeQuery1" false 0 "ForDuration" true "(R=1.000000,G=0.000000,B=0.000000,A=1.000000)" "(R=0.000000,G=1.000000,B=0.000000,A=1.000000)" 2.0))
  (if (and (.bBlockingHit (Collision|BreakHitResult _outhit)) (not (.bInitialOverlap (Collision|BreakHitResult _outhit))))
    (Utilities|FlowControl|DoOnce false :!label _label
      (:Completed
        (Default|HandleJumpandMantle _character)
        (Utilities|FlowControl|Delay 0.1)
        (Default|HandleJumpandMantle _character)
        (Utilities|FlowControl|Delay 0.5)
        (goto _label Reset)))))

(fn ConstructionScript)